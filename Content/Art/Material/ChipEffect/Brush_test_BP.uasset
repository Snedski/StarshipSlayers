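; Test Blueprint in the chip effect material folder that builds a cylinder brush from instanced meshes, with no active runtime logic.
; The construction script randomizes the instancing seed, then adds four instances, all using the component's own relative transform as their local transform.
; Each instance receives a custom data value stepping from zero to one, presumably read by the material to vary the coincident copies.
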(fn `UserConstructionScript`
  (bind _cylinder_brush (`self.Cylinder_Brush`))
  (bind _returnvalue (`SceneComponent.GetRelativeTransform` _cylinder_brush))
  (set `InstancedStaticMeshComponent.InstancingRandomSeed` (`KismetMathLibrary.RandomIntegerInRange` 1 12) _cylinder_brush)
  (bind _returnvalue_2 (`InstancedStaticMeshComponent.AddInstance` _cylinder_brush _returnvalue false))
  (`InstancedStaticMeshComponent.SetCustomDataValue` _cylinder_brush _returnvalue_2 0 0.0 false)
  (bind _returnvalue_3 (`InstancedStaticMeshComponent.AddInstance` _cylinder_brush _returnvalue false))
  (`InstancedStaticMeshComponent.SetCustomDataValue` _cylinder_brush _returnvalue_3 0 0.5 false)
  (bind _returnvalue_4 (`InstancedStaticMeshComponent.AddInstance` _cylinder_brush _returnvalue false))
  (`InstancedStaticMeshComponent.SetCustomDataValue` _cylinder_brush _returnvalue_4 0 1.0 false)
  (bind _returnvalue_5 (`InstancedStaticMeshComponent.AddInstance` _cylinder_brush _returnvalue false))
  (`InstancedStaticMeshComponent.SetCustomDataValue` _cylinder_brush _returnvalue_5 0 1.0 false))