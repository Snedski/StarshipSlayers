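; Interaction component that finds the interactable the player is looking at, focuses it with a HUD popup, and forwards Interact calls to it.
; Once set up with a camera, it sphere-traces forward each tick for WorldDynamic objects implementing InteractableInterface.
; A directly aimed-at candidate wins; otherwise the first one with clear line of sight from the camera is chosen.
; Focus messages notify interactables as focus is set or cleared.
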(event `self.ReceiveTick`
  (params (DeltaSeconds :type "Float (single-precision)"))
  (bind _cameraorigin (`self.CameraOrigin`))
  (bind _returnvalue (`SceneComponent.K2_GetComponentLocation` _cameraorigin))
  (`parent.ReceiveTick` DeltaSeconds)
  (bind (_outhits _returnvalue_2) (`KismetSystemLibrary.SphereTraceMultiForObjects` _returnvalue (+ _returnvalue (* (`SceneComponent.GetForwardVector` _cameraorigin) (`self.InteractionDistance`))) (`self.InteractionRadius`) (`|MakeArray` "ObjectTypeQuery2" :!type "EObjectTypeQuery Enum")))
  (if _returnvalue_2
    (bind _best_interactable (`self.Choose Best Interactable` _outhits))
    (`/Engine/EditorBlueprintResources/StandardMacros.IsValid` _best_interactable
      (:`Is Valid`
        (`|ExecutionSequence`
          (:`then_0`
            (`/Engine/EditorBlueprintResources/StandardMacros.IsValid` (`self.FocusedInteractable`)
              (:`Is Valid`
                (message `InteractableInterface.Focus` (`self.FocusedInteractable`) false))))
          (:`then_1`
            (bind _output_get (set `self.FocusedInteractable` _best_interactable))
            (message `InteractableInterface.Focus` _output_get true)
            (`MainHUD.ShowInteractionPopup` (`MainGameMode.GetHUD`) true))))
      (:`Is Not Valid`
        (`|ExecutionSequence` :!label _label
          (:`then_0`
            (`/Engine/EditorBlueprintResources/StandardMacros.IsValid` (`self.FocusedInteractable`)
              (:`Is Valid`
                (message `InteractableInterface.Focus` (`self.FocusedInteractable`) false)
                (set `self.FocusedInteractable` null))))
          (:`then_1`
            (`MainHUD.ShowInteractionPopup` (`MainGameMode.GetHUD`) false)))))
    (else
      (goto _label))))

(fn `Choose Best Interactable`
  (params (HitResults :type "Array of HitResult Structure"))
  (returns (`Best Interactable` :type "Actor Object Reference"))
  (locals (Best :type "Actor Object Reference") (PointAtResult :type "HitResult Structure") (IsPointingAtSomething :type Boolean :default false))
  (bind _cameraorigin (`self.CameraOrigin`))
  (bind (_bblockinghit _binitialoverlap _time _distance _location _impactpoint _normal _impactnormal _physmat _hitactor) (`GameplayStatics.BreakHitResult` (`local.PointAtResult`)))
  (bind _returnvalue (`SceneComponent.K2_GetComponentLocation` _cameraorigin))
  (`|ExecutionSequence`
    (:`then_0`
      (bind (_outhit _returnvalue_2) (`KismetSystemLibrary.LineTraceSingle` :`Start` _returnvalue :`End` (+ _returnvalue (* (`SceneComponent.GetForwardVector` _cameraorigin) 10000.0)) :`TraceChannel` "TraceTypeQuery1" :`TraceColor` (struct :`R` 1.0 :`B` 0.756586 :`A` 1.0)))
      (set `local.PointAtResult` _outhit)
      (set `local.IsPointingAtSomething` _returnvalue_2))
    (:`then_1`
      (for _array_element HitResults
        (bind (_bblockinghit_2 _binitialoverlap_2 _time_2 _distance_2 _location_2 _impactpoint_2 _normal_2 _impactnormal_2 _physmat_2 _hitactor_2) (`GameplayStatics.BreakHitResult` _array_element))
        (if (`KismetSystemLibrary.DoesImplementInterface` _hitactor_2 "/Script/StarshipSlayers.InteractableInterface")
          (if (and (`local.IsPointingAtSomething`) (== _hitactor _hitactor_2))
            (return _hitactor)
            (else
              (`/Engine/EditorBlueprintResources/StandardMacros.IsValid` (`local.Best`)
                (:`Is Not Valid`
                  (bind (_outhit_2 _returnvalue_3) (`KismetSystemLibrary.LineTraceSingle` :`Start` (`SceneComponent.K2_GetComponentLocation` (`self.CameraOrigin`)) :`End` (`Actor.K2_GetActorLocation` _hitactor_2) :`TraceChannel` "TraceTypeQuery1" :`TraceColor` (struct :`G` 0.114498 :`B` 1.0 :`A` 1.0)))
                  (bind (_bblockinghit_3 _binitialoverlap_3 _time_3 _distance_3 _location_3 _impactpoint_3 _normal_3 _impactnormal_3 _physmat_3 _hitactor_3) (`GameplayStatics.BreakHitResult` _outhit_2))
                  (if (and _returnvalue_3 (== _hitactor_3 _hitactor_2))
                    (set `local.Best` _hitactor_3))))))))
      (return (`local.Best`)))))

(fn `Interact`
  (bind _focusedinteractable (`self.FocusedInteractable`))
  (`/Engine/EditorBlueprintResources/StandardMacros.IsValid` _focusedinteractable
    (:`Is Valid`
      (message `InteractableInterface.Interact` _focusedinteractable))))

(fn `SetupSystem`
  (params (Camera :type "CameraComponent Object Reference"))
  (set `self.CameraOrigin` Camera)
  (`self.SetComponentTickEnabled` true))