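; Two-floor lift actor that slides a glass barrier vertically and carries its platform between floors.
; The outer trigger opens and closes the glass, while entering the inner trigger closes it and starts travel once shut; leaving before then reopens it.
; Tick drives both motions through a shared smoothing curve, reopening the glass on arrival.
; Triggers enable Tick, which switches itself off when glass movement finishes without a pending ride.
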(event `self.ReceiveBeginPlay`
  (`parent.ReceiveBeginPlay`)
  (set `self.CurrentFloor` (`self.StartingFloor`))
  (`SceneComponent.K2_SetRelativeLocation` (`self.Platform`) (`|GetArrayItem` (`self.Floors`) (`self.StartingFloor`)) false false))

(event `self.ReceiveTick`
  (params (DeltaSeconds :type "Float (single-precision)"))
  (`parent.ReceiveTick` DeltaSeconds)
  (`|ExecutionSequence`
    (:`then_0`
      (if (`self.GlassActive`)
        (`|ExecutionSequence`
          (:`then_0`
            (if (`self.GlassOpen`)
              (bind _output_get (set `self.CurrentGlassTransitionTime` (+ (`self.CurrentGlassTransitionTime`) DeltaSeconds)))
              (if (>= _output_get (`self.GlassTransitionTime`))
                (set `self.CurrentGlassTransitionTime` (`self.GlassTransitionTime`))
                (set `self.GlassActive` false)
                (`self.SetActorTickEnabled` false))
              (else
                (bind _output_get_2 (set `self.CurrentGlassTransitionTime` (- (`self.CurrentGlassTransitionTime`) DeltaSeconds)))
                (if (<= _output_get_2 0.0)
                  (set `self.CurrentGlassTransitionTime` 0.0)
                  (set `self.GlassActive` false)
                  (if (`self.ClosingLift`)
                    (set `self.ClosingLift` false)
                    (set `self.LiftActive` true)
                    (set `self.TargetFloor` (select `bool` (== (`self.CurrentFloor`) 0) :`true` 1))
                    (set `self.LiftTransitionTime` (/ (`KismetMathLibrary.Vector_Distance` (`SceneComponent.RelativeLocation` (`self.Platform`)) (`|GetArrayItem` (`self.Floors`) (`self.TargetFloor`))) (`self.LiftSpeed`)))
                    (set `self.CurrentLiftTransitionTime` 0.0)
                    (else
                      (`self.SetActorTickEnabled` false)))))))
          (:`then_1`
            (`SceneComponent.K2_SetRelativeLocation` (`self.Glass`) (`KismetMathLibrary.MakeVector` 0.0 0.0 (`KismetMathLibrary.Lerp` 0.0 300.0 (`KismetMathLibrary.FClamp` (`CurveFloat.GetFloatValue` (`self.SmoothCurve`) (/ (`self.CurrentGlassTransitionTime`) (`self.GlassTransitionTime`)))))) false false)))))
    (:`then_1`
      (if (`self.LiftActive`)
        (`|ExecutionSequence`
          (:`then_0`
            (bind _output_get_3 (set `self.CurrentLiftTransitionTime` (+ (`self.CurrentLiftTransitionTime`) DeltaSeconds)))
            (if (>= _output_get_3 (`self.LiftTransitionTime`))
              (set `self.CurrentLiftTransitionTime` (`self.LiftTransitionTime`))
              (set `self.LiftActive` false)
              (set `self.CurrentFloor` (`self.TargetFloor`))
              (set `self.GlassOpen` true)
              (set `self.GlassActive` true)))
          (:`then_1`
            (`SceneComponent.K2_SetRelativeLocation` (`self.Platform`) (`KismetMathLibrary.VLerp` (`|GetArrayItem` (`self.Floors`) (`self.CurrentFloor`)) (`|GetArrayItem` (`self.Floors`) (`self.TargetFloor`)) (`KismetMathLibrary.FClamp` (`CurveFloat.GetFloatValue` (`self.SmoothCurve`) (/ (`self.CurrentLiftTransitionTime`) (`self.LiftTransitionTime`))))) false false)))))))

(event `self.InnerTrigger.OnComponentBeginOverlap`
  (params (OverlappedComponent :type "PrimitiveComponent Object Reference") (OtherActor :type "Actor Object Reference") (OtherComp :type "PrimitiveComponent Object Reference") (OtherBodyIndex :type Integer) (bFromSweep :type Boolean) (SweepResult :type "HitResult Structure (by ref)"))
  (set `self.ClosingLift` true)
  (set `self.GlassOpen` false)
  (set `self.GlassActive` true)
  (`self.SetActorTickEnabled` true))

(event `self.InnerTrigger.OnComponentEndOverlap`
  (params (OverlappedComponent :type "PrimitiveComponent Object Reference") (OtherActor :type "Actor Object Reference") (OtherComp :type "PrimitiveComponent Object Reference") (OtherBodyIndex :type Integer))
  (if (`self.ClosingLift`)
    (set `self.ClosingLift` false)
    (set `self.GlassOpen` true)
    (set `self.GlassActive` true)
    (`self.SetActorTickEnabled` true)))

(event `self.OuterTrigger.OnComponentBeginOverlap`
  (params (OverlappedComponent :type "PrimitiveComponent Object Reference") (OtherActor :type "Actor Object Reference") (OtherComp :type "PrimitiveComponent Object Reference") (OtherBodyIndex :type Integer) (bFromSweep :type Boolean) (SweepResult :type "HitResult Structure (by ref)"))
  (set `self.GlassOpen` true)
  (set `self.GlassActive` true)
  (`self.SetActorTickEnabled` true))

(event `self.OuterTrigger.OnComponentEndOverlap`
  (params (OverlappedComponent :type "PrimitiveComponent Object Reference") (OtherActor :type "Actor Object Reference") (OtherComp :type "PrimitiveComponent Object Reference") (OtherBodyIndex :type Integer))
  (set `self.GlassOpen` false)
  (set `self.GlassActive` true)
  (`self.SetActorTickEnabled` true))

(fn `UserConstructionScript`)