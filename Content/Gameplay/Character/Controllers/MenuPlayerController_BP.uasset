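; Menu player controller Blueprint that passes any key press to DetectAnyKey, its only active logic.
; Debug print events for controller use, input mode and cursor visibility, including keyboard variants, are present but empty.
; Their PrintString chains remain in the graph but are disconnected, so none of them run.
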(event `self.PrintUsingController`
  (params (bUseController :type Boolean)))

(event `Key|AnyKey` :paused true
  (params (Key :type "Key Structure"))
  (:`Pressed`
    (`self.DetectAnyKey` Key)))

(event `self.PrintCurrentInputMode`
  (params (inputMode :type "ECurrentInputMode Enum" :default "CIM_GAME")))

(event `self.PrintKeyboardInputMode`
  (params (inputMode :type "ECurrentInputMode Enum" :default "CIM_GAME")))

(event `self.PrintMouseCursorVisibility`
  (params (bShow :type Boolean)))

(event `self.PrintKeyboardCursorVisibility`
  (params (bShow :type Boolean)))

(fn `UserConstructionScript`)