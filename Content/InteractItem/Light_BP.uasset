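; Light_BP is an interactable light actor that can be switched on and off in the game.
; TurnOn and TurnOff set the visibility of a RectLight and a Cube together and record the state in an On flag.
; ToggleLight reads that flag and calls the opposite event.
; The construction script is empty.
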(event `TurnOn`
  (`SceneComponent.SetVisibility` (`self.RectLight`) true false)
  (`SceneComponent.SetVisibility` (`self.Cube`) true false)
  (set `self.On` true))

(event `TurnOff`
  (`SceneComponent.SetVisibility` (`self.RectLight`) false false)
  (`SceneComponent.SetVisibility` (`self.Cube`) false false)
  (set `self.On` false))

(event `ToggleLight`
  (if (`self.On`)
    (`self.TurnOff`)
    (else
      (`self.TurnOn`))))

(fn `UserConstructionScript`)